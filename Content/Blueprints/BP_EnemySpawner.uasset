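; BP_EnemySpawner is a spawn-point actor that refills the level with BP_Enemy whenever none remain.
; On BeginPlay it gathers all spawners, prints their count, spawns a wave and starts a self-recalling two-second enemy check.
; Each wave gives every spawner location a 20% chance of an enemy, despite a comment saying 80%.
; Every placed instance runs this whole loop itself, covering all spawners rather than only its own location.
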(event `self.ReceiveBeginPlay`
  (bind _outactors (`GameplayStatics.GetAllActorsOfClass` "BP_EnemySpawner_C"))
  (`KismetSystemLibrary.PrintString` (`KismetStringLibrary.Concat_StrStr` "There are" (`KismetStringLibrary.Conv_IntToString` (`KismetArrayLibrary.Array_Length` _outactors)) "spawner in the level."))
  (`self.SpawnEnemies`)
  (`self.Check Enemy Count`))

(event `SpawnEnemies`
  (for _array_element (stale `self.ReceiveBeginPlay` _outactors)
    (if (> (`KismetMathLibrary.RandomFloat`) 0.8)
      (`|SpawnActorFromClass` "/Game/Blueprints/BP_Enemy.BP_Enemy_C" (`KismetMathLibrary.Conv_VectorToTransform` (`self.K2_GetActorLocation` _array_element)) "Undefined" "MultiplyWithRoot" null null))))

(event `Check Enemy Count`
  (bind _outactors (`GameplayStatics.GetAllActorsOfClass` "/Game/Blueprints/BP_Enemy.BP_Enemy_C"))
  (if (not (> (`KismetArrayLibrary.Array_Length` _outactors) 0))
    (`self.SpawnEnemies`))
  (`KismetSystemLibrary.Delay` 2.0)
  (`self.Check Enemy Count`))

(fn `UserConstructionScript`)