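; Enemy actor that gets a name and team material on spawn and dies when the player character touches it.
; BeginPlay fills an unset name or material from shuffled arrays, prints debug messages and applies the material to body and head.
; A looping 0.2-second Delay polls Health and destroys the actor at zero or below.
; Capsule overlap with BP_ThirdPersonCharacter sets Health negative, so the next poll removes it.
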(event `self.ReceiveBeginPlay`
  (bind _materials (`self.Materials`))
  (bind _names (`self.Names`))
  (`|ExecutionSequence`
    (:`then_0`
      ;[1 0 0.7039] Every .2 seconds, check to see if health <=0. If it is, destroy ourself
      (`KismetSystemLibrary.Delay` 0.2 :!label _label)
      (if (<= (`self.Health`) 0.0)
        (`self.K2_DestroyActor`)
        (else
          (goto _label))))
    (:`then_1`
      (if (== (`self.Enemy Name`) "None")
        (`KismetArrayLibrary.Array_Shuffle` _names)
        (set `self.Enemy Name` (`|GetArrayItem` _names)) ; Set to the randomized name
      )
      (`KismetSystemLibrary.PrintString` (`KismetStringLibrary.Concat_StrStr` (`KismetStringLibrary.Conv_NameToString` (`self.Enemy Name`)) "exits!")))
    (:`then_2`
      (`/Engine/EditorBlueprintResources/StandardMacros.IsValid` (`self.Enemy Team Material`)
        (:`Is Valid`
          (`KismetSystemLibrary.PrintString` "A mateirial have been set" true true (struct :`G` 1.0 :`B` 0.370887 :`A` 1.0)))
        (:`Is Not Valid`
          (`KismetSystemLibrary.PrintString` "Let's pick a random tool")
          (`KismetArrayLibrary.Array_Shuffle` _materials) ; Shuffle the material, pick the first one.
          (set `self.Enemy Team Material` (`|GetArrayItem` _materials))))
      (`PrimitiveComponent.SetMaterial` (`self.Body`) 0 (`self.Enemy Team Material`)) ; set the material that was selected
      (`PrimitiveComponent.SetMaterial` (`self.Head`) 0 (`self.Enemy Team Material`)))))

(event `self.Capsule.OnComponentBeginOverlap`
  (params (OverlappedComponent :type "PrimitiveComponent Object Reference") (OtherActor :type "Actor Object Reference") (OtherComp :type "PrimitiveComponent Object Reference") (OtherBodyIndex :type Integer) (bFromSweep :type Boolean) (SweepResult :type "HitResult Structure (by ref)"))
  (cast `/Game/ThirdPerson/Blueprints/BP_ThirdPersonCharacter` OtherActor) ; Did the player hit us?
  (set `self.Health` -1.0))

(fn `UserConstructionScript`)